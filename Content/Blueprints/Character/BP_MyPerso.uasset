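; BP_MyPerso is the player character, with movement, mouse look, jumping and a key-and-door interaction.
; The Interact input branches on the type of NearItem to either grab a key or try a door.
; A grabbed BP_MasterKey snaps to the mesh's KeySocket, and opens only its linked DoorToOpen, then is destroyed.
; Message events create and remove a WBP_MessageBox widget, which is also cleared on pickup.
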(event `InputAxis|Move Forward / Backward`
  (params (AxisValue :type "Float (single-precision)"))
  (bind (_returnvalue_roll _returnvalue_pitch _returnvalue_yaw) (`KismetMathLibrary.BreakRotator` (`self.GetControlRotation`)))
  ;[1 1 1] Character Movement
  (`self.AddMovementInput` (`KismetMathLibrary.GetForwardVector` (`KismetMathLibrary.MakeRotator` 0.0 0.0 _returnvalue_yaw)) AxisValue))

(event `InputAxis|Look Up / Down Mouse`
  (params (AxisValue :type "Float (single-precision)"))
  ;[1 1 1] Camera Movement
  (`self.AddControllerPitchInput` AxisValue))

(event `InputAxis|Turn Right / Left Mouse`
  (params (AxisValue :type "Float (single-precision)"))
  ;[1 1 1] Camera Movement
  (`self.AddControllerYawInput` AxisValue))

(event `InputAxis|Move Right / Left`
  (params (AxisValue :type "Float (single-precision)"))
  (bind (_returnvalue_roll _returnvalue_pitch _returnvalue_yaw) (`KismetMathLibrary.BreakRotator` (`self.GetControlRotation`)))
  ;[1 1 1] Character Movement
  (`self.AddMovementInput` (`KismetMathLibrary.GetRightVector` (`KismetMathLibrary.MakeRotator` 0.0 0.0 _returnvalue_yaw)) AxisValue))

(event `InputAction|Jump`
  (params (Key :type "Key Structure"))
  ;[1 1 1] Jump Action
  (:`Pressed`
    (`self.Jump`))
  (:`Released`
    (`self.StopJumping`)))

(event `DisplayMessageBox`
  (params (MessageToDisplay :type Text))
  ;[1 1 1] Display / Remove Message Box Widget
  (bind _returnvalue (`|CreateWidget` "/Game/Blueprints/UI/WBP_MessageBox.WBP_MessageBox_C" null MessageToDisplay))
  (bind _output_get (set `self.MessageBoxRef` _returnvalue))
  (`UserWidget.AddToViewport` _output_get 0))

(event `InputAction|Interact`
  (params (Key :type "Key Structure"))
  (bind _nearitem (`self.NearItem`))
  ;[1 1 1] Interact Action
  (:`Pressed`
    (`/Engine/EditorBlueprintResources/StandardMacros.IsValid` _nearitem
      (:`Is Valid`
        (switch `/Game/Blueprints/Items/E_TypeOfItem` (`/Game/Blueprints/Items/BP_ItemInteract.TypeOfItem` _nearitem)
          (:`NewEnumerator0`
            (`self.TryToOpenDoor`))
          (:`NewEnumerator1`
            (`self.GrabItem`)))))))

(event `RemoveMessageBox`
  ;[1 1 1] Display / Remove Message Box Widget
  (`Widget.RemoveFromParent` (`self.MessageBoxRef`)))

(event `TryToOpenDoor`
  (bind _doortoopen (`/Game/Blueprints/Items/BP_MasterKey.DoorToOpen` (`self.ItemEquipped`)))
  ;[1 1 1] Try to open door
  (if (`self.IsItemEquipped?`)
    (if (== _doortoopen (`self.NearItem`))
      (`/Game/Blueprints/Items/BP_MasterDoor.StartOpenDoor` _doortoopen)
      (`self.K2_DestroyActor` (`self.ItemEquipped`))
      (set `self.ItemEquipped` null))))

(event `GrabItem`
  ;[1 1 1] Get item near me
  (bind _asbp_master_key (cast `/Game/Blueprints/Items/BP_MasterKey` (`self.NearItem`)))
  (bind _output_get (set `self.ItemEquipped` _asbp_master_key))
  (set `self.IsItemEquipped?` true)
  (`SceneComponent.K2_AttachToComponent` (`Actor.RootComponent` _output_get) (`self.Mesh`) "KeySocket" "SnapToTarget" "SnapToTarget" "SnapToTarget" true)
  (`PrimitiveComponent.SetCollisionEnabled` (`/Game/Blueprints/Items/BP_ItemInteract.Mesh` _output_get) "NoCollision")
  (set `self.NearItem` null)
  (set `/Game/Blueprints/Items/BP_ItemInteract.IsInteractable` false _output_get)
  (`self.RemoveMessageBox`))

(fn `UserConstructionScript`)