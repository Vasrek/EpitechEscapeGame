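; BP_ItemInteract is an interactable item that shows the player an interaction prompt when they enter its Box trigger.
; On overlap, if IsInteractable is set, it builds a "Press E" message from TypeOfItem (Door, Key or Enigma) and NameOfItem.
; It passes the message to BP_MyPerso and registers itself as that character's NearItem.
; Leaving the box removes the message and clears NearItem.
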(event `self.Box.OnComponentBeginOverlap`
  (params (OverlappedComponent :type "PrimitiveComponent Object Reference") (OtherActor :type "Actor Object Reference") (OtherComp :type "PrimitiveComponent Object Reference") (OtherBodyIndex :type Integer) (bFromSweep :type Boolean) (SweepResult :type "HitResult Structure (by ref)"))
  ;[1 1 1] Display a message box along with the correct type of item
  (bind _asbp_my_perso (cast `/Game/Blueprints/Character/BP_MyPerso` OtherActor))
  (if (`self.IsInteractable`)
    (switch `/Game/Blueprints/Items/E_TypeOfItem` (`self.TypeOfItem`)
      (:`NewEnumerator0`
        (set `self.Format` "Press E to open "))
      (:`NewEnumerator1`
        (set `self.Format` "Press E to pick up "))
      (:`NewEnumerator2`
        (set `self.Format` "Press E to solve ")))
    (`/Game/Blueprints/Character/BP_MyPerso.DisplayMessageBox` _asbp_my_perso (`|FormatText` "{message} {nameofitem}" (`self.Format`) (`self.NameOfItem`)))
    (set `/Game/Blueprints/Character/BP_MyPerso.NearItem` self _asbp_my_perso)))

(event `self.Box.OnComponentEndOverlap`
  (params (OverlappedComponent :type "PrimitiveComponent Object Reference") (OtherActor :type "Actor Object Reference") (OtherComp :type "PrimitiveComponent Object Reference") (OtherBodyIndex :type Integer))
  ;[1 1 1] Remove the message box - Reset the variable near item ot nothing
  (bind _asbp_my_perso (cast `/Game/Blueprints/Character/BP_MyPerso` OtherActor))
  (`/Game/Blueprints/Character/BP_MyPerso.RemoveMessageBox` _asbp_my_perso)
  (set `/Game/Blueprints/Character/BP_MyPerso.NearItem` null _asbp_my_perso))

(fn `UserConstructionScript`)