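; BP_MasterDoor is a base-named door Blueprint that swings a cell door mesh open when StartOpenDoor runs.
; StartOpenDoor starts a fast looping timer on OpenDoor, which interpolates the mesh's world yaw toward a target, zeroing pitch and roll.
; Each tick subtracts a step from the interpolation speed.
; Once the next interpolated yaw is nearly at the target, the timer clears and the door stops being interactable.
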(event `StartOpenDoor`
  (`KismetSystemLibrary.K2_SetTimer` null "OpenDoor" 0.01 true))

(fn `OpenDoor`
  (bind (_returnvalue_roll _returnvalue_pitch _returnvalue_yaw) (`KismetMathLibrary.BreakRotator` (`SceneComponent.K2_GetComponentRotation` (`self.SM_Cell_Door`))))
  (bind _returnvalue (`KismetMathLibrary.FInterpTo` _returnvalue_yaw (`self.TargetToOpenDoor`) (`GameplayStatics.GetWorldDeltaSeconds`) (`self.InterpSpeed`)))
  (`SceneComponent.K2_SetWorldRotation` (`self.SM_Cell_Door`) (`KismetMathLibrary.MakeRotator` 0.0 0.0 _returnvalue) false false)
  (set `self.InterpSpeed` (- (`self.InterpSpeed`) (`self.InterpSpeedToAdd`)))
  (if (`KismetMathLibrary.NearlyEqual_FloatFloat` _returnvalue (`self.TargetToOpenDoor`) 5.0)
    (`KismetSystemLibrary.K2_ClearTimer` null "OpenDoor")
    (set `self.IsInteractable` false)))

(fn `UserConstructionScript`)